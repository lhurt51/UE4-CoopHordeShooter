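; Behavior tree service that picks the AI pawn's target actor in the horde shooter.
; On each AI tick it scans actors known through sight perception and keeps the nearest one that is not friendly and has health above zero in its SHealthComponent.
; The result is written to a configurable Blackboard key, which is cleared to None when no valid target lies within the maximum search distance.
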(event `self.ReceiveTickAI`
  (params (OwnerController :type "AIController Object Reference") (ControlledPawn :type "Pawn Object Reference") (DeltaSeconds :type "Float (single-precision)"))
  (set `self.BestTargetActor` null)
  (set `self.NearestTargetDst` 100000.0)
  (for _array_element (`AIPerceptionComponent.GetKnownPerceivedActors` (`Actor.GetComponentByClass` ControlledPawn "/Script/AIModule.AIPerceptionComponent") "/Script/AIModule.AISense_Sight")
    (bind _returnvalue (`KismetMathLibrary.VSize` (- (`Actor.K2_GetActorLocation` ControlledPawn) (`Actor.K2_GetActorLocation` _array_element))))
    (if (and (< _returnvalue (`self.NearestTargetDst`)) (not (`SHealthComponent.IsFriendly` _array_element ControlledPawn)) (> (`SHealthComponent.Health` (`Actor.GetComponentByClass` _array_element "/Script/CoopShooter.SHealthComponent")) 0.0))
      (set `self.NearestTargetDst` _returnvalue)
      (set `self.BestTargetActor` _array_element)))
  (`BTFunctionLibrary.SetBlackboardValueAsObject` (`self.BlackboardKey`) (`self.BestTargetActor`)))