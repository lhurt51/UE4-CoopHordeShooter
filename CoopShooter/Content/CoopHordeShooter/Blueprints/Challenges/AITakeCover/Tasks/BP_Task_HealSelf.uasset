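; Behavior tree task that lets an AI in the take-cover challenge heal its controlled pawn.
; It finds the pawn's SHealthComponent and applies two fixed-amount heals, each followed by a timed delay, then finishes successfully.
; Without a valid health component it calls FinishAbort rather than finishing as failed.
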(event `self.ReceiveExecuteAI`
  (params (OwnerController :type "AIController Object Reference") (ControlledPawn :type "Pawn Object Reference"))
  (bind _returnvalue (`Actor.GetComponentByClass` ControlledPawn "/Script/CoopShooter.SHealthComponent"))
  (`/Engine/EditorBlueprintResources/StandardMacros.IsValid` _returnvalue
    (:`Is Valid`
      (`SHealthComponent.Heal` _returnvalue (`self.HealPerTick`))
      (`KismetSystemLibrary.Delay` (`self.HealTickInterval`))
      (`SHealthComponent.Heal` _returnvalue (`self.HealPerTick`))
      (`KismetSystemLibrary.Delay` (`self.HealTickInterval`))
      (`self.FinishExecute` true))
    (:`Is Not Valid`
      (`self.FinishAbort`))))